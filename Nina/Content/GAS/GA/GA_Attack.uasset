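; GA_Attack is a Gameplay Ability that plays an attack montage from a random section, at the avatar RoleBase's attack rate.
; On activation it applies GE_CantMove to the owner, even if commit fails, and removes it when the ability ends.
; Montage events tagged Event.Montage apply the effect container matching their tag, passing along the event data.
; Blend out, interruption or cancellation of the montage ends the ability.
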(event `self.K2_ActivateAbility`
  (bind _montagetoplay (`self.MontageToPlay`))
  (bind _returnvalue (`self.K2_CommitAbility`))
  (bind _returnvalue_2 (`self.K2_ApplyGameplayEffectSpecToOwner` (`self.MakeOutgoingGameplayEffectSpec` "/Game/GAS/GE/GE_CantMove.GE_CantMove_C")))
  (set `self.StopMoveGEHandle` _returnvalue_2)
  (if _returnvalue
    (bind (_asynctaskproxy _eventtag _eventdata) (`RPGAbilityTask_PlayMontageAndWaitForEvent.PlayMontageAndWaitForEvent` "None" _montagetoplay (struct :`GameplayTags` (struct :`(TagName` "Event.Montage"))) (`RoleBase.GetAttackRate` (cast `RoleBase` (`self.GetAvatarActorFromActorInfo`) :!pure true)) (`AnimMontage.GetSectionName` _montagetoplay (`KismetMathLibrary.RandomInteger` (`AnimMontage.GetNumSections` _montagetoplay))))
      (:`OnBlendOut`
        (`self.K2_EndAbility` :!label _label))
      (:`OnInterrupted`
        (goto _label))
      (:`OnCancelled`
        (goto _label))
      (:`EventReceived`
        (`self.ApplyEffectContainer` _eventtag _eventdata) ; Immediately apply an effect container, it will normally use the event data for targeting
      ))))

(event `self.K2_OnEndAbility`
  (params (bWasCancelled :type Boolean))
  (`AbilitySystemComponent.RemoveActiveGameplayEffect` (`self.GetAbilitySystemComponentFromActorInfo`) (`self.StopMoveGEHandle`) -1))