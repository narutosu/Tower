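; Enemy character Blueprint whose mesh and animation class come from a RoleData primary asset, bound to a Lua module via GetModuleName.
; LuaImpUseRoleData force-loads that data and applies it in construction and BeginPlay; its comment says the Blueprint version runs only in-editor, implying a Lua runtime override.
; AI perception updates set IsFindPlayer by whether the actor is a BP_RoleHero, ignoring sense success.
; Attack activates slot 0 abilities.
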(event `self.ReceiveBeginPlay`
  (`self.LuaImp_UseRoleData`))

(event `self.AIPerception.OnTargetPerceptionUpdated`
  (params (Actor :type "Actor Object Reference") (Stimulus :type "AIStimulus Structure"))
  (cast `/Game/Blueprints/Characters/Hero/BP_RoleHero` Actor
    (:`then`
      (set `self.IsFindPlayer` true)
      (`KismetSystemLibrary.PrintString` "IsFindPlayer true"))
    (:`CastFailed`
      (set `self.IsFindPlayer` false)
      (`KismetSystemLibrary.PrintString` "IsFindPlayer false"))))

(fn `Attack`
  (`self.ActivateAbilitiesWithSlotNum` 0)
  (`KismetSystemLibrary.PrintString` "Attack"))

(fn `GetModuleName`
  (returns (ReturnValue :type String))
  (return "Characters.Enemy.BP_RoleEnemy_C"))

(fn `LuaImp_UseRoleData`
  (locals (RoleData :type "RoleData Object Reference"))
  ; 蓝图的实现只在Construct Script里调用。也就是只在编辑器下运行
  (bind _returnvalue (`RPGAssetManager.Get`))
  (bind _returnvalue_2 (`RPGAssetManager.ForceLoadItem` _returnvalue (`self.RoleDataID`) true))
  (bind _asrole_data (cast `RoleData` _returnvalue_2))
  (bind _output_get (set `local.RoleData` _asrole_data))
  (`/Engine/EditorBlueprintResources/StandardMacros.IsValid` _output_get
    (:`Is Valid`
      (`|ExecutionSequence`
        (:`then_0`
          ; SkeletalMesh
          (bind _returnvalue_3 (`KismetSystemLibrary.LoadAsset_Blocking` (`RoleData.SkeletalMesh` (`local.RoleData`))))
          (bind _asskeletal_mesh (cast `SkeletalMesh` _returnvalue_3))
          (`SkeletalMeshComponent.SetSkeletalMeshAsset` (`self.Mesh`) _asskeletal_mesh))
        (:`then_1`
          ; AnimInstance
          (bind _returnvalue_4 (`KismetSystemLibrary.LoadClassAsset_Blocking` (`RoleData.AnimInstance` (`local.RoleData`))))
          (`SkeletalMeshComponent.SetAnimInstanceClass` (`self.Mesh`) _returnvalue_4))))
    (:`Is Not Valid`
      (`KismetSystemLibrary.PrintString` "Cant  Find RoleData"))))

(fn `UserConstructionScript`
  (`self.LuaImp_UseRoleData`))